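; BP_Prop is a prop actor, stored with editor scripting utilities, that offers three functions for randomizing its look and placement.
; Random Mesh assigns one of six furniture, stair and bush meshes to its StaticMesh component.
; Random Rotation adds a random world yaw, and Random Offset nudges the actor slightly along its local X and Y axes.
; The event graph and construction script are empty, so nothing in the Blueprint calls these functions.
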(fn `Random Mesh`
  (`StaticMeshComponent.SetStaticMesh` (`self.StaticMesh`) (select `int` (`KismetMathLibrary.RandomIntegerInRange` 0 5) :`0` "/Game/StarterContent/Props/SM_Chair.SM_Chair" :`1` "/Game/StarterContent/Props/SM_Couch.SM_Couch" :`2` "/Game/VehicleVarietyPack/Meshes/SM_Lamp_Ceiling.SM_Lamp_Ceiling" :`3` "/Game/StarterContent/Props/SM_Stairs.SM_Stairs" :`4` "/Game/StarterContent/Props/SM_TableRound.SM_TableRound" :`5` "/Game/StarterContent/Props/SM_Bush.SM_Bush" :!type "StaticMesh Object Reference")))

(fn `Random Offset`
  (`self.K2_AddActorLocalOffset` (`KismetMathLibrary.MakeVector_NetQuantize` (`KismetMathLibrary.RandomFloatInRange` -20.0 20.0) (`KismetMathLibrary.RandomFloatInRange` -20.0 20.0))))

(fn `Random Rotation`
  (`self.K2_AddActorWorldRotation` (`KismetMathLibrary.MakeRotator` 0.0 0.0 (`KismetMathLibrary.RandomFloatInRange` 0.0 360.0))))

(fn `UserConstructionScript`)